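; Actor component that detects which BP_InteractionArea the player's camera is looking at and toggles that area's focus.
; Every tick it line-traces on the Visibility channel along camera forward for a configurable length.
; When the hit actor changes, an exact class check decides whether to unfocus the previous area and focus the new one.
; A miss or other actor type unfocuses and clears the current area.
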(event EventTick
  (params (DeltaSeconds :type Float%20%28single-precision%29))
  (CallFunction|Trace))

(fn Trace
  (bind _returnvalue (Game|GetPlayerCameraManager 0))
  (bind _returnvalue_2 (Transformation|GetActorLocation _returnvalue))
  (bind (_outhit _returnvalue_3) (Collision|LineTraceByChannel _returnvalue_2 (+ _returnvalue_2 (* (Math|Vector|GetForwardVector (Transformation|GetActorRotation _returnvalue)) (Variables|Default|GetLength))) "TraceTypeQuery1" false 0 "None"))
  (if _returnvalue_3
    ;[0.05098 0.05098 0.05098] If the hit actor is not the focus actor
    (if (!= (Variables|Default|GetFocusedActor) (.HitActor (Collision|BreakHitResult _outhit)))
      ;[0.05098 0.05098 0.05098] Set the actor that is focus
      (Variables|Default|SetFocusedActor (.HitActor (Collision|BreakHitResult _outhit)))
      (CallFunction|TraceInteractionArea (== (Utilities|GetClass (.HitActor (Collision|BreakHitResult _outhit))) "/Game/RenovationSimulator/Blueprints/Interactions/BP_InteractionArea.BP_InteractionArea_C")))
    (else
      (CallFunction|TraceInteractionArea false))))

(fn TraceInteractionArea
  (params (Trace :type Boolean))
  (if Trace
    (if (Variables|Default|GetIsTracingInteractionArea)
      ;[0.05098 0.05098 0.05098] Unfocus
      (Variables|Default|GetFocusedInteractionArea
        (:then
          (Default|ToggleFocus (Variables|Default|GetFocusedInteractionArea) false))
        (:else)))
    (bind _asbp_interaction_area (Utilities|Casting|CastToBP_InteractionArea (Variables|Default|GetFocusedActor)))
    (bind _output_get (Variables|Default|SetFocusedInteractionArea _asbp_interaction_area))
    (Default|ToggleFocus _output_get true)
    (Variables|Default|SetIsTracingInteractionArea true)
    (elif (Variables|Default|GetIsTracingInteractionArea)
      (Variables|Default|SetIsTracingInteractionArea false)
      (Variables|Default|GetFocusedInteractionArea
        (:then
          (Default|ToggleFocus (Variables|Default|GetFocusedInteractionArea) false)
          ;[0.05098 0.05098 0.05098] Set to null
          (Variables|Default|SetFocusedActor 0)
          (Variables|Default|SetFocusedInteractionArea 0))
        (:else)))))