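; Farming crop actor that grows day by day through BP_TimeDay's OnDay event, swapping meshes from sprout to grown using PlantData.
; Unwatered days stall growth, and a third consecutive one kills the plant.
; A Delay-throttled Tick sets the interaction prompt from growth stage and the player's tool.
; When focused, IA_Interact waters the plant or removes it, spawning a BP_ROTFPlantTile in its place.
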(event Input|EnhancedActionEvents|EnhancedInputActionIA_Interact
  (params (ActionValue :type Boolean) (ElapsedSeconds :type Float%20%28double-precision%29) (TriggeredSeconds :type Float%20%28double-precision%29) (InputAction :type Input%20Action%20Object%20Reference :default "/Game/Character/Input/Actions/IA_Interact.IA_Interact"))
  (:Started
    (if (Variables|Interaction|GetFocus)
      (switch Utilities|FlowControl|Switch|SwitchonE_StageOfGrowth (Variables|Plant|GetStageOfGrowth)
        (:NewEnumerator1
          (switch name (Variables|/Game/Character/Blueprints/BP_ROTFCharacter.BP_ROTFCharacter_C|GetCurrentTool (Variables|Default|GetPlayer))
            (:Tool_03
              (Utilities|RemovePlant))
            (:Tool_04
              (if (and (Default|CanUseWateringCan (Variables|Default|GetPlayer)) (not (Variables|Plant|GetWateredToday)))
                (CallFunction|WaterPlant)))))
        (:NewEnumerator2
          (Utilities|RemovePlant))
        (:NewEnumerator3
          (if (== (Variables|/Game/Character/Blueprints/BP_ROTFCharacter.BP_ROTFCharacter_C|GetCurrentTool (Variables|Default|GetPlayer)) "Tool_02")
            (Utilities|RemovePlant)))))))

(event EventBeginPlay
  ;[0.05098 0.05098 0.05098] Initialization
  (bind _asbp_rotfcharacter (Utilities|Casting|CastToBP_ROTFCharacter (Game|GetPlayerCharacter 0)))
  (Variables|Default|SetPlayer _asbp_rotfcharacter)
  (bind _aswbp_rotf_interaction_input (Utilities|Casting|CastToWBP_ROTF_Interaction_Input (UserInterface|GetUserWidgetObject (Variables|Default|GetWidget))))
  (bind _output_get (Variables|Interaction|SetInteractionInputWidget _aswbp_rotf_interaction_input))
  (Default|SetMessage _output_get "" true)
  (bind _outactors (Actor|GetAllActorsOfClass "/Game/RenovationSimulator/Blueprints/BP_TimeDay.BP_TimeDay_C"))
  (bind _output_get_2 (Variables|Default|SetTimeDay (Utilities|Array|Get(acopy) _outactors)))
  (EventDispatchers|BindEventtoOnDay _output_get_2 (EventDispatchers|CreateEvent :!event Growing)))

(event EventTick
  (params (DeltaSeconds :type Float%20%28single-precision%29))
  (Utilities|FlowControl|Delay 0.5)
  ;[0.05098 0.05098 0.05098] Action name
  (switch Utilities|FlowControl|Switch|SwitchonE_StageOfGrowth (Variables|Plant|GetStageOfGrowth)
    (:NewEnumerator1
      (switch name (Variables|/Game/Character/Blueprints/BP_ROTFCharacter.BP_ROTFCharacter_C|GetCurrentTool (Variables|Default|GetPlayer))
        (:Default
          (Default|SetMessage (Variables|Interaction|GetInteractionInputWidget) "" true))
        (:Tool_03
          (Default|SetMessage (Variables|Interaction|GetInteractionInputWidget) "Dig it up" true))
        (:Tool_04
          (if (Variables|Plant|GetWateredToday)
            (Default|SetMessage (Variables|Interaction|GetInteractionInputWidget) "Watered today" false)
            (elif (Default|CanUseWateringCan (Variables|Default|GetPlayer))
              (Default|SetMessage (Variables|Interaction|GetInteractionInputWidget) "Water plant" true)
              (else
                (Default|SetMessage (Variables|Interaction|GetInteractionInputWidget) "Not enough water" false)))))))
    (:NewEnumerator2
      (if (== (Variables|/Game/Character/Blueprints/BP_ROTFCharacter.BP_ROTFCharacter_C|GetCurrentTool (Variables|Default|GetPlayer)) "Tool_03")
        (Default|SetMessage (Variables|Interaction|GetInteractionInputWidget) "Dig it up" true)
        (else
          (Default|SetMessage (Variables|Interaction|GetInteractionInputWidget) "Collect" true))))
    (:NewEnumerator3
      (if (== (Variables|/Game/Character/Blueprints/BP_ROTFCharacter.BP_ROTFCharacter_C|GetCurrentTool (Variables|Default|GetPlayer)) "Tool_02")
        (Default|SetMessage (Variables|Interaction|GetInteractionInputWidget) "Remove" true)
        (else
          (Default|SetMessage (Variables|Interaction|GetInteractionInputWidget) "" true))))))

(event EventInterfaceToggleFocus
  (params (Focus :type Boolean))
  ;[0.05098 0.05098 0.05098] Toggle Focus Event
  (Variables|Interaction|SetFocus Focus))

(fn ConstructionScript)

(fn GetRandomMesh
  (params (Meshes :type Array%20of%20Static%20Mesh%20Object%20References))
  (return (Utilities|Array|Get(acopy) Meshes (Math|Random|RandomInteger (Utilities|Array|Length Meshes)))))

(fn SetStageOfGrowth
  (params (NewStageOfGrowth :type E_StageOfGrowth%20Enum :default "NewEnumerator0"))
  (Variables|Plant|SetStageOfGrowth NewStageOfGrowth)
  (return))

(fn UnbindGrowing
  (EventDispatchers|UnbindEventfromOnDay (Variables|Default|GetTimeDay) (EventDispatchers|CreateEvent :!event Growing)))

(fn SetInteractionAreaScale
  (params (Scale :type Vector))
  (bind _bp_rotfinteractionarea (Variables|Default|GetBP_ROTFInteractionArea))
  (Transformation|SetRelativeScale3D _bp_rotfinteractionarea (Math|Vector|MakeVector (.x Scale) (.y Scale) (.z Scale)))
  (Transformation|SetRelativeLocation _bp_rotfinteractionarea (Math|Vector|MakeVector 0.0 0.0 (* (- (.z Scale) 0.2) 32.0)) false false))

(fn WaterPlant
  (Variables|Plant|SetDaysWithoutWater 0)
  (Math|Integer|DecrementInt (Variables|/Game/Character/Blueprints/BP_ROTFCharacter.BP_ROTFCharacter_C|GetWateringCanUses (Variables|Default|GetPlayer))
    (:%20%20
      (Variables|Plant|SetWateredToday true))))

(fn Growing
  (bind _plantdata (Variables|Plant|GetPlantData))
  (bind _plantmesh (Variables|Default|GetPlantMesh))
  (Utilities|IncrementDaysWithoutWater
    (:NotDead
      (Variables|Plant|SetDays (+ (Variables|Plant|GetDays) (Variables|Plant|GetGrowthPerDay)))
      (Variables|Plant|SetGrowthPerDay 1)
      (Variables|Plant|SetWateredToday false)
      (if (== (Variables|Plant|GetDays) 1)
        (Components|StaticMesh|SetStaticMesh (Variables|Default|GetPlantMesh) (CallFunction|GetRandomMesh (Variables|Plant|GetSproutMeshes)))
        (elif (== (Variables|Plant|GetDays) (Utilities|Array|Get(acopy) (.growtime (Variables|Plant|GetPlantData))))
          (Components|StaticMesh|SetStaticMesh _plantmesh (.startermesh _plantdata))
          (Transformation|SetRelativeScale3D _plantmesh (.meshscale _plantdata))
          (CallFunction|SetInteractionAreaScale (.hitboxscale _plantdata))
          (elif (== (Variables|Plant|GetDays) (Utilities|Array|Get(acopy) (.growtime (Variables|Plant|GetPlantData)) 1))
            (Components|StaticMesh|SetStaticMesh (Variables|Default|GetPlantMesh) (CallFunction|GetRandomMesh (.grownupmesh (Variables|Plant|GetPlantData))))
            (CallFunction|UnbindGrowing)
            (Variables|Plant|SetStageOfGrowth "NewEnumerator2")))))))

(fn InterfaceWidgetInput
  (return (Variables|Default|GetWidget)))