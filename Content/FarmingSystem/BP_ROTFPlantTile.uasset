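; BP_ROTFPlantTile is a farming plot where the player plants seeds, replacing itself with a BP_ROTFPlant.
; Its prompt widget shows "Plant {seed name}" while Seeds are the current tool, refreshed through a half-second Delay on Tick.
; Interacting while focused spawns the plant on the tile's parent, consumes a seed and destroys the tile.
; Plant data comes from a name search of DT_ROTF_Plants, falling back to Plant_01.
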(event Input|EnhancedActionEvents|EnhancedInputActionIA_Interact
  (params (ActionValue :type Boolean) (ElapsedSeconds :type Float%20%28double-precision%29) (TriggeredSeconds :type Float%20%28double-precision%29) (InputAction :type Input%20Action%20Object%20Reference :default "/Game/Character/Input/Actions/IA_Interact.IA_Interact"))
  (bind _player (Variables|Default|GetPlayer))
  (:Started
    (if (and (Variables|Interaction|GetFocus) (== (Variables|/Game/Character/Blueprints/BP_ROTFCharacter.BP_ROTFCharacter_C|GetCurrentTool (Variables|Default|GetPlayer)) "Seeds"))
      (Audio|PlaySound2D "/Game/Sounds/click.click" 1.0 1.0 0.0 0 0)
      (bind _returnvalue (Game|SpawnActorfromClass "/Game/FarmingSystem/BP_ROTFPlant.BP_ROTFPlant_C" (Transformation|GetActorTransform) "Undefined" "MultiplyWithRoot" 0 0))
      (Transformation|AttachActorToActor _returnvalue (Actor|GetAttachParentActor) "None" "KeepWorld" "KeepRelative" "KeepRelative" true)
      (Default|RemoveOneSeed _player)
      (bind _plantdata (CallFunction|FindPlantbyName (Variables|/Game/Character/Blueprints/BP_ROTFCharacter.BP_ROTFCharacter_C|GetSeedsName _player)))
      (Variables|/Game/FarmingSystem/BP_ROTFPlant.BP_ROTFPlant_C|SetPlantData _returnvalue _plantdata)
      (Actor|DestroyActor))))

(event EventBeginPlay
  ;[0.05098 0.05098 0.05098] Initialization
  (bind _asbp_rotfcharacter (Utilities|Casting|CastToBP_ROTFCharacter (Game|GetPlayerCharacter 0)))
  (Variables|Default|SetPlayer _asbp_rotfcharacter)
  (bind _aswbp_rotf_interaction_input (Utilities|Casting|CastToWBP_ROTF_Interaction_Input (UserInterface|GetUserWidgetObject (Variables|Default|GetWidget))))
  (bind _output_get (Variables|Interaction|SetInteractionInputWidget _aswbp_rotf_interaction_input))
  (Default|SetMessage _output_get "" true))

(event EventInterfaceToggleFocus
  (params (Focus :type Boolean))
  ;[0.05098 0.05098 0.05098] Toggle Focus Event
  (Variables|Interaction|SetFocus Focus))

(event EventTick
  (params (DeltaSeconds :type Float%20%28single-precision%29))
  (Utilities|FlowControl|Delay 0.5)
  ;[0.05098 0.05098 0.05098] Action name
  (if (== (Variables|/Game/Character/Blueprints/BP_ROTFCharacter.BP_ROTFCharacter_C|GetCurrentTool (Variables|Default|GetPlayer)) "Seeds")
    (Default|SetMessage (Variables|Interaction|GetInteractionInputWidget) (Utilities|Text|FormatText "Plant {plantName}" (Variables|/Game/Character/Blueprints/BP_ROTFCharacter.BP_ROTFCharacter_C|GetSeedsName (Variables|Default|GetPlayer))) true)
    (else
      (Default|SetMessage (Variables|Interaction|GetInteractionInputWidget) "" true))))

(fn ConstructionScript)

(fn FindPlantbyName
  (params (PlantName :type Name))
  (bind _outrownames (DataTable|GetDataTableRowNames "/Game/DataStucture/Databases/DT_ROTF_Plants.DT_ROTF_Plants"))
  (for _array_element _outrownames
    (bind _returnvalue (Utilities|GetDataTableRow "/Game/DataStucture/Databases/DT_ROTF_Plants.DT_ROTF_Plants" _array_element)
      (:then
        (if (== (.Name (Utilities|Struct|BreakF_Plant _returnvalue)) PlantName)
          (return _returnvalue)))))
  (bind _returnvalue_2 (Utilities|GetDataTableRow "/Game/DataStucture/Databases/DT_ROTF_Plants.DT_ROTF_Plants" "Plant_01")
    (:then
      (return _returnvalue_2))))

(fn InterfaceWidgetInput
  (return (Variables|Default|GetWidget)))