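; BP_LightsControl switches tagged night lights in the level according to the time of day.
; On BeginPlay it binds handlers to the 18:00 and 8:00 events of the first BP_TimeDay actor found.
; NightLightsOn and NightLightsOff set fixed or zero intensity on "Home" spot lights and "Plane" point lights.
; The point-light pass is nested inside the spot-light loop, so it repeats per spot light.
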(event EventBeginPlay
  (bind _outactors (Actor|GetAllActorsOfClass "/Game/RenovationSimulator/Blueprints/BP_TimeDay.BP_TimeDay_C"))
  (EventDispatchers|BindEventtoOn18Hour (Utilities|Array|Get(acopy) _outactors) (EventDispatchers|CreateEvent :!event NightLightson))
  (EventDispatchers|BindEventtoOn8Hour (Utilities|Array|Get(acopy) _outactors) (EventDispatchers|CreateEvent :!event NightLightsOff)))

(fn ConstructionScript)

(fn NightLightson
  (bind _outactors (Actor|GetAllActorsOfClasswithTag "/Script/Engine.SpotLight" "Home"))
  (for _array_element _outactors
    (Rendering|Components|Light|SetIntensity (Variables|/Script/Engine.SpotLight|GetSpotLightComponent _array_element) 3.0)
    (bind _outactors_2 (Actor|GetAllActorsOfClasswithTag "/Script/Engine.PointLight" "Plane"))
    (for _array_element_2 _outactors_2
      (Rendering|Components|Light|SetIntensity (Variables|/Script/Engine.PointLight|GetPointLightComponent _array_element_2) 4.0))))

(fn NightLightsOff
  (bind _outactors (Actor|GetAllActorsOfClasswithTag "/Script/Engine.SpotLight" "Home"))
  (for _array_element _outactors
    (Rendering|Components|Light|SetIntensity (Variables|/Script/Engine.SpotLight|GetSpotLightComponent _array_element) 0.0)
    (bind _outactors_2 (Actor|GetAllActorsOfClasswithTag "/Script/Engine.PointLight" "Plane"))
    (for _array_element_2 _outactors_2
      (Rendering|Components|Light|SetIntensity (Variables|/Script/Engine.PointLight|GetPointLightComponent _array_element_2) 0.0))))