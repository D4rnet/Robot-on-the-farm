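; BP_ROTFWaterPit is an interactable water pit where the player refills the watering can.
; It caches the player character and its interaction prompt widget, which a delayed Tick refreshes to show "Collect water" only while Tool_04 is equipped.
; An interface event tracks focus, and IA_Interact resets the can to maximum uses when the pit is focused and that tool is held.
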(event Input|EnhancedActionEvents|EnhancedInputActionIA_Interact
  (params (ActionValue :type Boolean) (ElapsedSeconds :type Float%20%28double-precision%29) (TriggeredSeconds :type Float%20%28double-precision%29) (InputAction :type Input%20Action%20Object%20Reference :default "/Game/Character/Input/Actions/IA_Interact.IA_Interact"))
  (if (and (Variables|Interaction|GetFocus) (== (Variables|/Game/Character/Blueprints/BP_ROTFCharacter.BP_ROTFCharacter_C|GetCurrentTool (Variables|Default|GetPlayer)) "Tool_04"))
    (Default|SetMaxWateringCanUses (Variables|Default|GetPlayer))))

(event EventTick
  (params (DeltaSeconds :type Float%20%28single-precision%29))
  (Utilities|FlowControl|Delay 0.5)
  (if (== (Variables|/Game/Character/Blueprints/BP_ROTFCharacter.BP_ROTFCharacter_C|GetCurrentTool (Variables|Default|GetPlayer)) "Tool_04")
    (Default|SetMessage (Variables|Interaction|GetInteractionInputWidget) "Collect water" true)
    (else
      (Default|SetMessage (Variables|Interaction|GetInteractionInputWidget) "" false))))

(event EventInterfaceToggleFocus
  (params (Focus :type Boolean))
  ;[0.05098 0.05098 0.05098] Toggle Focus Event
  (Variables|Interaction|SetFocus Focus))

(event EventBeginPlay
  ;[0.05098 0.05098 0.05098] Initialization
  (bind _asbp_rotfcharacter (Utilities|Casting|CastToBP_ROTFCharacter (Game|GetPlayerCharacter 0)))
  (Variables|Default|SetPlayer _asbp_rotfcharacter)
  (bind _aswbp_rotf_interaction_input (Utilities|Casting|CastToWBP_ROTF_Interaction_Input (UserInterface|GetUserWidgetObject (Variables|Default|GetWidget))))
  (bind _output_get (Variables|Interaction|SetInteractionInputWidget _aswbp_rotf_interaction_input))
  (if (== (Variables|/Game/Character/Blueprints/BP_ROTFCharacter.BP_ROTFCharacter_C|GetCurrentTool (Variables|Default|GetPlayer)) "Tool_04")
    (Default|SetMessage _output_get "Collect water" true)))

(fn ConstructionScript)

(fn InterfaceWidgetInput
  (return (Variables|Default|GetWidget)))