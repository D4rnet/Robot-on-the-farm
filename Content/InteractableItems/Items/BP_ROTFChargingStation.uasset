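; Interactable charging station that lets the ROTF player charge while time fast-forwards to 8:00 of the next day.
; When focused, interact disables input, flags charging, fades the HUD out and moves the player to the station's location and rotation.
; SpeedUpTimeTo8Hours temporarily overrides BP_TimeDay's day length for a computed delay instead of setting the clock.
; It then restores the day length, fades in and re-enables input.
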(event Input|EnhancedActionEvents|EnhancedInputActionIA_Interact
  (params (ActionValue :type Boolean) (ElapsedSeconds :type Float%20%28double-precision%29) (TriggeredSeconds :type Float%20%28double-precision%29) (InputAction :type Input%20Action%20Object%20Reference :default "/Game/Character/Input/Actions/IA_Interact.IA_Interact"))
  (:Started
    (if (and (Variables|Interaction|GetFocus) (Default|IsinGameWidget (Variables|Default|GetHUD)))
      (Input|DisableInput (Variables|Default|GetPlayer) (Game|GetPlayerController 0))
      (Variables|/Game/Character/Blueprints/BP_ROTFCharacter.BP_ROTFCharacter_C|SetIsCharging (Variables|Default|GetPlayer) true)
      (bind _animationtime (Default|PlayFadeOutAnimation (Variables|Default|GetHUD)))
      (Utilities|FlowControl|Delay _animationtime)
      (Transformation|SetActorLocation (Variables|Default|GetPlayer) (Transformation|GetActorLocation) false false)
      (Pawn|SetControlRotation (Game|GetPlayerController 0) (Transformation|GetActorRotation))
      (Utilities|SpeedUpTimeto8Hours)
      (Default|PlayFadeinAnimation (Variables|Default|GetHUD))
      (Variables|/Game/Character/Blueprints/BP_ROTFCharacter.BP_ROTFCharacter_C|SetIsCharging (Variables|Default|GetPlayer) false)
      (Input|EnableInput (Variables|Default|GetPlayer) (Game|GetPlayerController 0)))))

(event EventBeginPlay
  (bind _aswbp_rotf_interaction_input (Utilities|Casting|CastToWBP_ROTF_Interaction_Input (UserInterface|GetUserWidgetObject (Variables|Default|GetWidget))))
  (bind _output_get (Variables|Interaction|SetInteractionInputWidget _aswbp_rotf_interaction_input))
  (Default|SetMessage _output_get "Charge" true)
  ;[0.05098 0.05098 0.05098] Get HUD
  (bind _asbp_rotfhud (Utilities|Casting|CastToBP_ROTFHUD (HUD|GetHUD (Game|GetPlayerController 0))))
  (Variables|Default|SetHUD _asbp_rotfhud)
  (bind _outactors (Actor|GetAllActorsOfClass "/Game/RenovationSimulator/Blueprints/BP_TimeDay.BP_TimeDay_C"))
  (Variables|Day/Nightcycle|SetTimeDay (Utilities|Array|Get(acopy) _outactors))
  (bind _asbp_rotfcharacter (Utilities|Casting|CastToBP_ROTFCharacter (Game|GetPlayerCharacter 0)))
  (Variables|Default|SetPlayer _asbp_rotfcharacter))

(event EventInterfaceToggleFocus
  (params (Focus :type Boolean))
  (Variables|Interaction|SetFocus Focus))

(fn ConstructionScript)

(fn InterfaceWidgetInput
  (return (Variables|Default|GetWidget)))