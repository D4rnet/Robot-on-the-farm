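; BP_ROTFDoor is an interactable door that swings open and closed when the player presses Interact while it has focus.
; Separate open and close timelines lerp the door's yaw using OpenDoorAngle, with InProgress blocking retriggers and Closed selecting the direction.
; An interface event sets focus, and another interface function exposes the prompt widget.
; Tick, throttled by a half-second Delay, switches the prompt between "Open door" and "Close door".
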(event Custom|OpenDoorEvent
  ;[0.05098 0.05098 0.05098] Open Door Event
  (Variables|Door|SetInProgress true)
  (bind _doorfloat_ (Timeline|OpenDoorTimeline PlayFromStart)
    (:Update
      (Transformation|SetRelativeRotation (Variables|Default|GetDoor) (Math|Rotator|MakeRotator 0.0 0.0 (Math|Float|Lerp 0.0 (Variables|Door|GetOpenDoorAngle) _doorfloat_)) false false))
    (:Finished
      (Variables|Door|SetClosed false)
      (Variables|Door|SetInProgress false))))

(event Custom|CloseDoorEvent
  ;[0.05098 0.05098 0.05098] Close Door Event
  (Variables|Door|SetInProgress true)
  (bind _doorfloat_ (Timeline|CloseDoorTimeline PlayFromStart)
    (:Update
      (Transformation|SetRelativeRotation (Variables|Default|GetDoor) (Math|Rotator|MakeRotator 0.0 0.0 (Math|Float|Lerp 0.0 (Variables|Door|GetOpenDoorAngle) _doorfloat_)) false false))
    (:Finished
      (Variables|Door|SetClosed true)
      (Variables|Door|SetInProgress false))))

(event Input|EnhancedActionEvents|EnhancedInputActionIA_Interact
  (params (ActionValue :type Boolean) (ElapsedSeconds :type Float%20%28double-precision%29) (TriggeredSeconds :type Float%20%28double-precision%29) (InputAction :type Input%20Action%20Object%20Reference :default "/Game/Character/Input/Actions/IA_Interact.IA_Interact"))
  (:Started
    (if (Variables|Interaction|GetFocus)
      (if (not (Variables|Door|GetInProgress))
        (if (Variables|Door|GetClosed)
          (CallFunction|OpenDoorEvent)
          (else
            (CallFunction|CloseDoorEvent)))))))

(event EventBeginPlay
  (bind _aswbp_rotf_interaction_input (Utilities|Casting|CastToWBP_ROTF_Interaction_Input (UserInterface|GetUserWidgetObject (Variables|Default|GetWidget))))
  (Variables|/Game/UI/Widgets/Childs/WBP_ROTF_Interaction_Input.WBP_ROTF_Interaction_Input_C|SetAction _aswbp_rotf_interaction_input "Open door"))

(event EventInterfaceToggleFocus
  (params (Focus :type Boolean))
  ;[0.05098 0.05098 0.05098] Toggle Focus Event
  (Variables|Interaction|SetFocus Focus))

(event EventTick
  (params (DeltaSeconds :type Float%20%28single-precision%29))
  (Utilities|FlowControl|Delay 0.5)
  ;[0.05098 0.05098 0.05098] Action name
  (if (Variables|Door|GetClosed)
    (bind _aswbp_rotf_interaction_input (Utilities|Casting|CastToWBP_ROTF_Interaction_Input (UserInterface|GetUserWidgetObject (Variables|Default|GetWidget))))
    (Variables|/Game/UI/Widgets/Childs/WBP_ROTF_Interaction_Input.WBP_ROTF_Interaction_Input_C|SetAction _aswbp_rotf_interaction_input "Open door")
    (else
      (bind _aswbp_rotf_interaction_input_2 (Utilities|Casting|CastToWBP_ROTF_Interaction_Input (UserInterface|GetUserWidgetObject (Variables|Default|GetWidget))))
      (Variables|/Game/UI/Widgets/Childs/WBP_ROTF_Interaction_Input.WBP_ROTF_Interaction_Input_C|SetAction _aswbp_rotf_interaction_input_2 "Close door"))))

(fn ConstructionScript)

(fn InterfaceWidgetInput
  (return (Variables|Default|GetWidget)))