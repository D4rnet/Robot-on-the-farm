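; Day/night cycle actor for Renovation Simulator that drives the game clock, sun and night sky.
; Each tick it advances a timespan clock, firing OnDay when the day changes, and rotates the directional light at a DayLength-scaled rate.
; The sun's pitch selects day or night lighting, which eases sun and skylight intensities toward targets and sets night-sky glow and opacity from that pitch.
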(event Custom|DayUpdate)

(event EventBeginPlay
  ;[0.05098 0.05098 0.05098] Initialization
  (bind _asbp_first_person_character (Utilities|Casting|CastToBP_FirstPersonCharacter (Game|GetPlayerCharacter 0)))
  (Variables|Default|SetPlayer _asbp_first_person_character))

(event EventTick
  (params (DeltaSeconds :type Float%20%28single-precision%29))
  (bind _directionallight (Variables|Day/NightCycle|GetDirectionalLight))
  (bind _day_length (Variables|Day/NightCycle|GetDay_Length))
  (bind _returnvalue (* DeltaSeconds _day_length))
  ;[0.05098 0.05098 0.05098] Day/night cycle
  ;;[0.1255 0.1255 0.1255] Hours/Days
  (CallFunction|Clock _returnvalue)
  (Transformation|AddActorLocalRotation _directionallight (Math|Rotator|MakeRotator 0.0 _returnvalue 0.0) false false)
  ;;[0.1255 0.1255 0.1255] If it's night
  (bind _output_get (Variables|Day/NightCycle|SetNight_Time (Math|Float|InRange(Float) (.pitch (Transformation|GetActorRotation _directionallight)) 0.0 1e+02)))
  (if _output_get
    (CallFunction|NightLighting _returnvalue)
    (else
      (CallFunction|DayLighting _returnvalue))))

(fn ConstructionScript)

(fn DayLighting
  (params (Delta :type Float%20%28double-precision%29))
  (bind _returnvalue (/ Delta 64.0))
  (bind _directionallight (Variables|Day/NightCycle|GetDirectionalLight))
  (bind _directionallight_2 (Variables|Day/NightCycle|GetDirectionalLight))
  (bind _skylight (Variables|Day/NightCycle|GetSkyLight))
  (bind _night_sky (Variables|Day/NightCycle|GetNight%20sky))
  (bind _returnvalue_2 (Transformation|GetActorRotation _directionallight_2))
  (bind _lightcomponent (Variables|/Script/Engine.Light|GetLightComponent _directionallight))
  (bind _lightcomponent_2 (Variables|/Script/Engine.SkyLight|GetLightComponent _skylight))
  (bind _staticmeshcomponent (Variables|/Script/Engine.StaticMeshActor|GetStaticMeshComponent _night_sky))
  (bind _returnvalue_3 (/ (.pitch _returnvalue_2) 9e+01))
  (bind _returnvalue_4 (+ _returnvalue_3 0.1))
  (bind _returnvalue_5 (/ _returnvalue_4 2.0))
  (Rendering|Components|Light|SetIntensity _lightcomponent (Math|Interpolation|FInterpTo (Variables|/Script/Engine.LightComponentBase|GetIntensity _lightcomponent) 3.0 _returnvalue 4.0))
  (Rendering|Components|Light|SetIntensity _lightcomponent_2 (Math|Interpolation|FInterpTo (Variables|/Script/Engine.LightComponentBase|GetIntensity _lightcomponent_2) 0.4 _returnvalue 8.0))
  (Rendering|Material|SetScalarParameterValueonMaterials _staticmeshcomponent "GlowCrank" (* _returnvalue_5 1.0))
  (Rendering|Material|SetScalarParameterValueonMaterials _staticmeshcomponent "Opacity" (* _returnvalue_5 0.5)))

(fn NightLighting
  (params (Delta :type Float%20%28double-precision%29))
  (bind _returnvalue (/ Delta 64.0))
  (bind _directionallight (Variables|Day/NightCycle|GetDirectionalLight))
  (bind _directionallight_2 (Variables|Day/NightCycle|GetDirectionalLight))
  (bind _skylight (Variables|Day/NightCycle|GetSkyLight))
  (bind _night_sky (Variables|Day/NightCycle|GetNight%20sky))
  (bind _returnvalue_2 (Transformation|GetActorRotation _directionallight_2))
  (bind _lightcomponent (Variables|/Script/Engine.Light|GetLightComponent _directionallight))
  (bind _lightcomponent_2 (Variables|/Script/Engine.SkyLight|GetLightComponent _skylight))
  (bind _staticmeshcomponent (Variables|/Script/Engine.StaticMeshActor|GetStaticMeshComponent _night_sky))
  (bind _returnvalue_3 (/ (.pitch _returnvalue_2) 9e+01))
  (bind _returnvalue_4 (+ _returnvalue_3 0.1))
  (bind _returnvalue_5 (/ _returnvalue_4 2.0))
  (Rendering|Components|Light|SetIntensity _lightcomponent (Math|Interpolation|FInterpTo (Variables|/Script/Engine.LightComponentBase|GetIntensity _lightcomponent) 0.3 _returnvalue 3.0))
  (Rendering|Components|Light|SetIntensity _lightcomponent_2 (Math|Interpolation|FInterpTo (Variables|/Script/Engine.LightComponentBase|GetIntensity _lightcomponent_2) 0.2 _returnvalue 5e+01))
  (Rendering|Material|SetScalarParameterValueonMaterials _staticmeshcomponent "GlowCrank" (* _returnvalue_5 1.0))
  (Rendering|Material|SetScalarParameterValueonMaterials _staticmeshcomponent "Opacity" (* _returnvalue_5 0.5)))

(fn Clock
  (params (Delta :type Float%20%28double-precision%29))
  (bind _output_get (Variables|Hours/Days|SetTick (+ (* Delta 2.4e+02) (Variables|Hours/Days|GetTick))))
  (Variables|Hours/Days|SetTime (Math|Timespan|MakeTimespan 1 12 0 (Math|Float|Truncate _output_get)))
  (if (!= (Variables|Default|GetPrevious%20day) (Math|Timespan|GetDays (Math|Timespan|MakeTimespan 1 12 0 (Math|Float|Truncate _output_get))))
    (Variables|Default|SetPrevious%20day (Math|Timespan|GetDays (Math|Timespan|MakeTimespan 1 12 0 (Math|Float|Truncate _output_get))))
    (Default|CallOnDay)))