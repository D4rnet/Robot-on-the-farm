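; BP_Chest is an interactable chest whose lid swings open when a pickup is triggered on it.
; MulticastPickup runs the parent logic, enables Tick and binds PickedUp to the pickup event dispatcher.
; While interactable, Tick waits a one-time delay to open a Gate, then pitches ChestTop one degree per frame up to 90, so speed follows frame rate.
; PickedUp disables Tick and further interaction.
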(event Custom|Picked%20Up
  (Actor|Tick|SetActorTickEnabled false)
  (Variables|Default|Set⚙%20Can%20Interact? false))

(event EventMulticastPickup
  (params (Object%20Pickup :type Actor%20Object%20Reference) (Location :type Actor%20Object%20Reference))
  (|CallParentFunction Object%20Pickup Location)
  (Actor|Tick|SetActorTickEnabled true)
  (EventDispatchers|AssignEDPickup (delegate Custom|Picked%20Up)))

(event EventTick
  (params (DeltaSeconds :type Float%20%28single-precision%29))
  (bind _chest_top (Variables|Default|GetChest%20Top))
  (bind _relativerotation (Variables|/Script/Engine.SceneComponent|GetRelativeRotation _chest_top))
  (bind _pitch (Math|Rotator|BreakRotator _relativerotation))
  (if (Variables|Default|Get⚙%20Can%20Interact?)
    (if (< _pitch 9e+01)
      (Utilities|FlowControl|Sequence
        (:then_0
          (Utilities|FlowControl|DoOnce false
            (:Completed
              (Utilities|FlowControl|Delay (Variables|Default|GetDelay%20To%20Open%20Chest))
              (goto _label Open))))
        (:then_1
          (Utilities|FlowControl|Gate true :!label _label
            (:Exit
              (Transformation|SetRelativeRotation _chest_top (Math|Rotator|MakeRotator 0.0 (+ _pitch 1.0) 0.0) false false))))))
    (else
      (Actor|Tick|SetActorTickEnabled false))))

(fn ConstructionScript
  (|CallParentFunction))